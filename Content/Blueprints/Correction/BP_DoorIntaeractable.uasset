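; Interactable door Blueprint that opens and closes by instantly moving its Cube component between a raised and a lowered relative position.
; Activate toggles the door based on the cube's current height, while InitializeState calls Open or Close for the Activated or Deactivated state.
; BeginPlay stores GetState's result in State; GetState checks the height but always returns Activated, overwriting the derived value.
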(event EventBeginPlay
  (bind _actualstate (CallFunction|GetState))
  (Variables|Default|SetState _actualstate))

(event Collision|EventActorBeginOverlap
  (params (OtherActor :type Actor%20Object%20Reference)))

(event EventTick
  (params (DeltaSeconds :type Float%20%28single-precision%29)))

(event EventActivate
  (CallFunction|ToggleOpenCloseDoor))

(event EventInitializeState
  (params (InitialState :type BPE_InteractableStates%20Enum :default "NewEnumerator0"))
  (switch Utilities|FlowControl|Switch|SwitchonBPE_InteractableStates InitialState
    (:NewEnumerator0
      (CallFunction|Open))
    (:NewEnumerator1
      (CallFunction|Close))))

(fn ConstructionScript)

(fn ToggleOpenCloseDoor
  (bind _cube (Variables|Default|GetCube))
  ;[1 1 1] Ferme ou ouvre la porte
  (if (> (.z (Variables|/Script/Engine.SceneComponent|GetRelativeLocation _cube)) 1.6e+02)
    (Transformation|SetRelativeLocation _cube "0.000000,0.000000,150.000000" false false)
    (else
      (Transformation|SetRelativeLocation _cube "0.000000,0.000000,400.000000" false false))))

(fn GetState
  (if (> (.z (Variables|/Script/Engine.SceneComponent|GetRelativeLocation (Variables|Default|GetCube))) 1.6e+02)
    (Variables|Default|SetState "NewEnumerator0")
    (else
      (Variables|Default|SetState "NewEnumerator1")))
  (return "NewEnumerator0"))

(fn Open
  (Transformation|SetRelativeLocation (Variables|Default|GetCube) "0.000000,0.000000,400.000000" false false))

(fn Close
  (Transformation|SetRelativeLocation (Variables|Default|GetCube) "0.000000,0.000000,150.000000" false false))