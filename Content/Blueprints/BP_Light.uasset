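; BP_Light is a light actor that switches on when three doors are closed.
; Its Activate event increments a closed-door counter and toggles the PointLight on when the count reaches exactly three.
; Its Deactivate event decrements the counter and turns the light off if it is visible.
; ToggleLight simply inverts the PointLight's visibility; BeginPlay, overlap and Tick do nothing.
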(event EventBeginPlay)

(event Collision|EventActorBeginOverlap
  (params (OtherActor :type Actor%20Object%20Reference)))

(event EventTick
  (params (DeltaSeconds :type Float%20%28single-precision%29)))

(event EventActivate
  (CallFunction|IsLightActivable))

(event EventDeactivate
  (CallFunction|IsLightDeactivable))

(fn ConstructionScript)

(fn ToggleLight
  (bind _pointlight (Variables|Default|GetPointLight))
  ;[1 1 1] Allume la lumière.
  (Rendering|SetVisibility _pointlight (not (Variables|/Script/Engine.SceneComponent|GetbVisible _pointlight)) false))

(fn IsLightActivable
  (bind _doorclosed (Variables|Default|GetDoorClosed))
  ;[1 1 1] Vérifie le nombre de portes fermées. S'il y en a 3, la lumière s'allume.
  (Math|Integer|IncrementInt _doorclosed
    (:%20%20
      (if (== _doorclosed 3)
        (CallFunction|ToggleLight)))))

(fn IsLightDeactivable
  ;[1 1 1] Vérifie le nombre de portes fermées. Si la lumière est allumée, alors elle s'éteint.
  (Math|Integer|DecrementInt (Variables|Default|GetDoorClosed)
    (:%20%20
      (if (Rendering|IsVisible (Variables|Default|GetPointLight))
        (CallFunction|ToggleLight)))))