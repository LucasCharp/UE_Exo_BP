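; BP_DoorDrivenByEvent is a door that toggles between open and closed when an external event launcher fires.
; On BeginPlay it binds its OpenAndClose event to the EventLauncher's ActivateControllables dispatcher.
; OpenAndClose calls OpenCloseDoor, which checks the mesh's relative height and snaps it to the raised or lowered position without animation or sweep.
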(event Custom|OpenAndClose
  (CallFunction|OpenCloseDoor))

(event EventBeginPlay
  (EventDispatchers|BindEventtoActivateControllables (Variables|Default|GetEventLauncher) (delegate Custom|OpenAndClose)))

(event Collision|EventActorBeginOverlap
  (params (OtherActor :type Actor%20Object%20Reference)))

(event EventTick
  (params (DeltaSeconds :type Float%20%28single-precision%29)))

(fn ConstructionScript)

(fn OpenCloseDoor
  (bind _sm_door (Variables|Default|GetSM_Door))
  (if (> (.z (Variables|/Script/Engine.SceneComponent|GetRelativeLocation _sm_door)) 1.6e+02)
    (Transformation|SetRelativeLocation _sm_door "60.000000,5.000000,150.000000" false false)
    (else
      (Transformation|SetRelativeLocation _sm_door "60.000000,5.000000,400.000000" false false))))