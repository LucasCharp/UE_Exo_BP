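; Door Blueprint whose Open event toggles a mesh between lowered and raised positions and notifies a linked controllable.
; Open calls OpenCloseDoor only if BPControllables implements BPI_InterrupteurContollable.
; OpenCloseDoor infers the state from SMDoor's relative height and snaps it to the other position without interpolation or sweep.
; Lowering sends ActivateMessage to BPControllables, while raising sends DeactivateMessage.
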(event EventBeginPlay)

(event Collision|EventActorBeginOverlap
  (params (OtherActor :type Actor%20Object%20Reference)))

(event EventTick
  (params (DeltaSeconds :type Float%20%28single-precision%29)))

(event EventOpen
  (if (Utilities|DoesObjectImplementInterface (Variables|Default|GetBP_Controllables) "/Game/Blueprints/BPI_InterrupteurContollable.BPI_InterrupteurContollable_C")
    (CallFunction|OpenCloseDoor)))

(fn ConstructionScript)

(fn OpenCloseDoor
  (bind _sm_door (Variables|Default|GetSM_Door))
  ;[1 1 1] Ferme ou ouvre la porte
  (if (> (.z (Variables|/Script/Engine.SceneComponent|GetRelativeLocation _sm_door)) 1.6e+02)
    (Transformation|SetRelativeLocation _sm_door "60.000000,5.000000,150.000000" false false)
    (Class|BPIInterrupteurContollable|Activate(Message) (Variables|Default|GetBP_Controllables))
    (else
      (Transformation|SetRelativeLocation _sm_door "60.000000,5.000000,400.000000" false false)
      (Class|BPIInterrupteurContollable|Deactivate(Message) (Variables|Default|GetBP_Controllables)))))